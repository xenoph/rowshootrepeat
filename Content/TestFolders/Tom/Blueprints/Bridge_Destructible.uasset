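; Destructible bridge actor that loses health when a trace calls its TakeDamage event and breaks apart at zero health.
; Each hit briefly spikes the emissive strength of a dynamic material created at BeginPlay, then a short timer lowers it again.
; At zero health it applies radius damage to fracture its DestructibleComponent and starts a looping one-second counter that destroys the actor once it exceeds RemovalTimer.
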(event `ChangeEmission`
  (`MaterialInstanceDynamic.SetScalarParameterValue` (`self.DynMaterial`) "Emissive Strength" 10.0))

(event `self.ReceiveBeginPlay`
  (bind _returnvalue (`PrimitiveComponent.CreateDynamicMaterialInstance` (`self.DestructibleComponent`) 0 (`PrimitiveComponent.GetMaterial` (`self.DestructibleComponent`) 0)))
  (set `self.DynMaterial` _returnvalue))

(event `/Game/TestFolders/BV/Blueprints/Interfaces/IShootable.TakeDamage`
  (params (DamageTaken :type "Float (single-precision)"))
  ;[1 1 1] Called from the trace
  (bind _output_get (set `self.Health` (- (`self.Health`) DamageTaken)))
  (`|ExecutionSequence`
    (:`then_0`
      ;[1 1 1] Check if broken
      (if (<= _output_get 0.0)
        ;[1 1 1] Apply damage to break the mesh
        (`DestructibleComponent.ApplyRadiusDamage` (`self.DestructibleComponent`) 1.0 (`SceneComponent.K2_GetComponentLocation` (`self.DestructibleComponent`)) 1.0 0.0 true)
        ;[1 1 1] Destroy Actor after set time
        (`KismetSystemLibrary.K2_SetTimerDelegate` (delegate `AddToCounter`) 1.0 true)))
    (:`then_1`
      (`MaterialInstanceDynamic.SetScalarParameterValue` (`self.DynMaterial`) "Emissive Strength" 400.0)
      (`KismetSystemLibrary.K2_SetTimerDelegate` (delegate `ChangeEmission`) 0.3))))

(event `AddToCounter`
  ;[1 1 1] Destroy Actor after set time
  (bind _result (`/Engine/EditorBlueprintResources/StandardMacros.IncrementFloat` (`self.Counter`))
    (:`  `
      (if (> _result (`self.RemovalTimer`))
        (`self.K2_DestroyActor`)))))

(fn `UserConstructionScript`)