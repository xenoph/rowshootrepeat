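; BP_EnemyCube2 is an enemy cube that bobs up and down while homing in on the player pawn.
; Tick alternates vertical offsets by frame counters, using a random bob step, and moves it toward the player by Speed and stored delta time.
; On BeginPlay, a splittable cube spawns copies along Y, flags them as SplittingMob and shrinks itself.
; The random SplittingMob roll does not gate that spawning.
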(event `self.ReceiveBeginPlay`
  (`|ExecutionSequence`
    (:`then_0`
      (bind _output_get (set `self.BopFloatUp` (`KismetMathLibrary.RandomFloatInRange` 1.0 4.0)))
      (bind _result (`/Engine/EditorBlueprintResources/StandardMacros.NegateFloat` _output_get)
        (:`  `
          (set `self.BopFloatDown` _result))))
    (:`then_1`
      (if (`self.SplittingMob`)
        (`SceneComponent.SetWorldScale3D` (`self.StaticMeshComponent`) (0.25 0.25 0.25))
        (set `self.Speed` 100.0)
        (`KismetSystemLibrary.PrintString` "Hello")
        (elif (`self.CanBeSplit`)
          (`|ExecutionSequence`
            (:`then_0`
              (if (< (`KismetMathLibrary.RandomIntegerInRange` 0 5) 5)
                (set `self.SplittingMob` false)
                (else
                  (set `self.SplittingMob` true))))
            (:`then_1`
              (if (`self.SplittingMob`)
                _
                (else
                  _))
              (for _ (range 3)
                (`|ExecutionSequence`
                  (:`then_0`
                    (`self.CreateSplitTransformArray`))
                  (:`then_1`
                    (bind _returnvalue (`|SpawnActorFromClass` "BP_EnemyCube2_C" (`KismetMathLibrary.Conv_VectorToTransform` (`KismetArrayLibrary.Array_Get` (`self.SplitTransformArray`) (`self.ArrayLoopCount`))) "Undefined" "OverrideRootScale"))
                    (`/Engine/EditorBlueprintResources/StandardMacros.IncrementInt` (`self.ArrayLoopCount`)
                      (:`  `
                        (set `/Game/TestFolders/BV/Blueprints/BP_EnemyCube2.SplittingMob` true _returnvalue)
                        (`KismetSystemLibrary.PrintString` (`KismetStringLibrary.Conv_VectorToString` (`self.K2_GetActorLocation` _returnvalue)) true true (struct :`G` 0.66 :`B` 1.0 :`A` 1.0) 15.0))))))
              (`SceneComponent.SetWorldScale3D` (`self.StaticMeshComponent`) (0.25 0.25 0.25)))))))))

(event `self.ReceiveTick`
  (params (DeltaSeconds :type "Float (single-precision)"))
  (bind _returnvalue (`self.K2_GetActorLocation`))
  (`|ExecutionSequence`
    (:`then_0`
      ;[1 1 1] Bop the enemy up and down
      (if (< (`self.UpCounter`) 100)
        (`self.K2_AddActorLocalOffset` (`KismetMathLibrary.MakeVector` 0.0 0.0 (`self.BopFloatUp`)))
        (set `self.UpCounter` (+ (`self.UpCounter`) 1))
        (else
          (`self.K2_AddActorLocalOffset` (`KismetMathLibrary.MakeVector` 0.0 0.0 (`self.BopFloatDown`)))
          (bind _output_get (set `self.DownCounter` (+ (`self.DownCounter`) 1)))
          (if (== _output_get 100)
            (`|ExecutionSequence`
              (:`then_0`
                (set `self.UpCounter` 0))
              (:`then_1`
                (set `self.DownCounter` 0)))))))
    (:`then_1`
      ;[1 1 1] Move the enemy towards the player
      (`self.K2_SetActorLocation` (+ (* (* (`KismetMathLibrary.Normal` (- (`self.K2_GetActorLocation` (`GameplayStatics.GetPlayerPawn` 0)) _returnvalue)) (`self.Tick`)) (`self.Speed`)) _returnvalue)))
    (:`then_2`
      (set `self.Tick` DeltaSeconds))))

(fn `UserConstructionScript`)