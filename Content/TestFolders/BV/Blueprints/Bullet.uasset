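; Player bullet Blueprint that destroys enemies on overlap and expires after a short fixed lifespan set on BeginPlay.
; On actor overlap it checks for an exact class match with the flying enemy or the land-enemy projectile, prints a debug message, then destroys both that actor and itself.
; An older Hit-based version of the check remains disconnected and never runs.
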(event `self.ReceiveHit`
  (params (MyComp :type "PrimitiveComponent Object Reference") (Other :type "Actor Object Reference") (OtherComp :type "PrimitiveComponent Object Reference") (bSelfMoved :type Boolean) (HitLocation :type "Vector Structure") (HitNormal :type "Vector Structure") (NormalImpulse :type "Vector Structure") (Hit :type "HitResult Structure (by ref)")))

(event `self.ReceiveBeginPlay`
  (`|ExecutionSequence`
    (:`then_0`
      (`self.SetLifeSpan` 2.5))))

(event `self.ReceiveActorBeginOverlap`
  (params (OtherActor :type "Actor Object Reference"))
  (bind _output_get (set `self.HitObject` OtherActor))
  (`|ExecutionSequence`
    (:`then_0`
      (bind _returnvalue (`GameplayStatics.GetObjectClass` _output_get))
      (if (or (== _returnvalue "/Game/TestFolders/BV/Blueprints/Enemies/BP_FlyingEnemy1.BP_FlyingEnemy1_C") (== _returnvalue "/Game/TestFolders/BV/Blueprints/Enemies/BP_Projectile_LandEnemy.BP_Projectile_LandEnemy_C"))
        (`|ExecutionSequence`
          (:`then_0`
            (`KismetSystemLibrary.PrintString` "You hit an enemy"))
          (:`then_1`
            (`self.K2_DestroyActor` (`self.HitObject`)))
          (:`then_2`
            (`self.K2_DestroyActor`)))))))

(fn `UserConstructionScript`)