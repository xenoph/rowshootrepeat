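; Breakable cracked cave stalagmite that takes damage from a trace and drops once its health runs out.
; TakeDamage lowers Health, enables gravity on the mesh at zero, and briefly spikes the emissive strength of a dynamic material as damage feedback, with a timer lowering it again.
; A Hit event starts a looping one-second counter that destroys the actor once it exceeds TimeToDestroy.
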(event `self.ReceiveBeginPlay`
  (bind _returnvalue (`PrimitiveComponent.CreateDynamicMaterialInstance` (`self.StaticMeshComponent`) 0 (`PrimitiveComponent.GetMaterial` (`self.StaticMeshComponent`) 0)))
  (set `self.DynMaterial` _returnvalue))

(event `ChangeEmission`
  (`MaterialInstanceDynamic.SetScalarParameterValue` (`self.DynMaterial`) "Emissive Strength" 10.0))

(event `/Game/TestFolders/BV/Blueprints/Enemies/IShootable.TakeDamage`
  (params (DamageTaken :type "Float (single-precision)"))
  ;[1 1 1] Called from the trace
  (bind _output_get (set `self.Health` (- (`self.Health`) DamageTaken)))
  (`|ExecutionSequence`
    (:`then_0`
      ;[1 1 1] Check if broken
      (if (<= _output_get 0.0)
        (`PrimitiveComponent.SetEnableGravity` (`self.StaticMeshComponent`) true)))
    (:`then_1`
      (`MaterialInstanceDynamic.SetScalarParameterValue` (`self.DynMaterial`) "Emissive Strength" 400.0)
      (`KismetSystemLibrary.K2_SetTimerDelegate` (delegate `ChangeEmission`) 0.3))))

(event `self.ReceiveHit`
  (params (MyComp :type "PrimitiveComponent Object Reference") (Other :type "Actor Object Reference") (OtherComp :type "PrimitiveComponent Object Reference") (bSelfMoved :type Boolean) (HitLocation :type "Vector Structure") (HitNormal :type "Vector Structure") (NormalImpulse :type "Vector Structure") (Hit :type "HitResult Structure (by ref)"))
  ;[1 1 1] Destroy Actor after set time
  (`KismetSystemLibrary.K2_SetTimerDelegate` (delegate `AddToCounter`) 1.0 true))

(event `AddToCounter`
  ;[1 1 1] Destroy Actor after set time
  (bind _result (`/Engine/EditorBlueprintResources/StandardMacros.IncrementFloat` (`self.Counter`))
    (:`  `
      (if (> _result (`self.TimeToDestroy`))
        (`self.K2_DestroyActor`)))))

(fn `UserConstructionScript`)