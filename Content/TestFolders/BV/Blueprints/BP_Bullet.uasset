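; BP_Bullet is a projectile actor that damages or destroys enemies it overlaps.
; On overlap, it matches the other actor's exact class against a hardcoded list of flying enemy, land enemy and land enemy projectile classes.
; Flying enemies lose Health by Damage, and both they and the bullet are destroyed only when Health runs out.
; Land enemies and their projectiles are destroyed immediately along with the bullet.
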(event `self.ReceiveActorBeginOverlap`
  (params (OtherActor :type "Actor Object Reference"))
  (bind _output_get (set `self.HitObject` OtherActor))
  (for _array_element (`|MakeArray` "/Game/TestFolders/BV/Blueprints/Enemies/BP_FlyingEnemy1.BP_FlyingEnemy1_C" "/Game/TestFolders/BV/Blueprints/Enemies/BP_Projectile_LandEnemy.BP_Projectile_LandEnemy_C" "/Game/TestFolders/BV/Blueprints/Enemies/BP_LandEnemy.BP_LandEnemy_C" :!type "Object Class Reference")
    (bind _returnvalue (`GameplayStatics.GetObjectClass` _output_get))
    (if (== _array_element _returnvalue)
      (if (== _returnvalue "/Game/TestFolders/BV/Blueprints/Enemies/BP_FlyingEnemy1.BP_FlyingEnemy1_C")
        (bind _asbp_flying_enemy_1 (cast `/Game/TestFolders/BV/Blueprints/Enemies/BP_FlyingEnemy1` (`self.HitObject`)))
        (bind _output_get_2 (set `/Game/TestFolders/BV/Blueprints/Enemies/BP_FlyingEnemy1.Health` (- (`/Game/TestFolders/BV/Blueprints/Enemies/BP_FlyingEnemy1.Health` _asbp_flying_enemy_1) (`self.Damage`)) _asbp_flying_enemy_1))
        (if (<= _output_get_2 0.0)
          (`self.K2_DestroyActor` (`self.HitObject`))
          (`self.K2_DestroyActor`))
        (else
          (`|ExecutionSequence`
            (:`then_0`
              (`self.K2_DestroyActor` (`self.HitObject`)))
            (:`then_1`
              (`self.K2_DestroyActor`))))))))

(event `self.ReceiveBeginPlay`
  (`/Engine/EditorBlueprintResources/StandardMacros.NegateFloat` (`self.Damage`)))

(fn `UserConstructionScript`)