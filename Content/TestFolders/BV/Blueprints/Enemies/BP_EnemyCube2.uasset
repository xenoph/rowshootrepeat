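; Cube enemy that homes in on the player pawn, with optional bobbing and splitting into smaller copies.
; On BeginPlay it randomizes the bob offset and, if splittable, spawns quarter-scale copies along Y, flagged against re-splitting, and shrinks itself.
; The random split roll does not gate spawning.
; Tick alternates counter-based bob phases and steps toward the player at Speed, scaled by delta time, without sweep.
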(event `self.ReceiveBeginPlay`
  (bind _bopuprange (`self.BopUpRange`))
  (bind (_returnvalue_location _returnvalue_rotation) (`KismetMathLibrary.BreakTransform` (`KismetMathLibrary.Conv_VectorToTransform` (`KismetArrayLibrary.Array_Get` (`self.SplitTransformArray`) (`self.ArrayLoopCount`)))))
  (`|ExecutionSequence`
    (:`then_0`
      ;[1 1 1] Set Bopping range. At least Array0, at most Array1
      (if (`self.BopUpAndDown`)
        (bind _output_get (set `self.BopFloatUp` (`KismetMathLibrary.RandomFloatInRange` (`KismetArrayLibrary.Array_Get` _bopuprange) (`KismetArrayLibrary.Array_Get` _bopuprange 1))))
        (`/Engine/EditorBlueprintResources/StandardMacros.NegateFloat` _output_get
          (:`  `
            (set `self.BopFloatDown` 0.0)))))
    (:`then_1`
      ;[1 1 1] Split the enemy up. Tidy up this shit you slob
      (`|ExecutionSequence`
        (:`then_1`
          (if (`self.SplittingMob`)
            _
            (elif (`self.CanBeSplit`)
              (`|ExecutionSequence`
                (:`then_0`
                  (if (< (`KismetMathLibrary.RandomIntegerInRange` 0 5) 5)
                    (set `self.SplittingMob` false)
                    (else
                      (set `self.SplittingMob` true))))
                (:`then_1`
                  (if (`self.SplittingMob`)
                    _
                    (else
                      _))
                  (for _ (range 3)
                    (`|ExecutionSequence`
                      (:`then_0`
                        (`self.CreateSplitTransformArray`))
                      (:`then_1`
                        (bind _returnvalue (`|SpawnActorFromClass` "BP_EnemyCube2_C" (`KismetMathLibrary.MakeTransform` _returnvalue_location _returnvalue_rotation (0.25 0.25 0.25)) "Undefined" "OverrideRootScale"))
                        (`/Engine/EditorBlueprintResources/StandardMacros.IncrementInt` (`self.ArrayLoopCount`)
                          (:`  `
                            (set `/Game/TestFolders/BV/Blueprints/Enemies/BP_EnemyCube2.SplittingMob` true _returnvalue)
                            (`KismetSystemLibrary.PrintString` (`KismetStringLibrary.Conv_VectorToString` (`self.K2_GetActorLocation` _returnvalue)) true true (struct :`G` 0.66 :`B` 1.0 :`A` 1.0) 15.0))))))
                  (`SceneComponent.SetWorldScale3D` (`self.StaticMeshComponent`) (0.25 0.25 0.25)))))))))))

(event `self.ReceiveTick`
  (params (DeltaSeconds :type "Float (single-precision)"))
  (bind _returnvalue (`self.K2_GetActorLocation`))
  (set `self.Tick` DeltaSeconds)
  (`|ExecutionSequence`
    (:`then_0`
      ;[1 1 1] Bop the enemy up and down
      (if (`self.BopUpAndDown`)
        (if (< (`self.UpCounter`) 100)
          (`self.K2_AddActorLocalOffset` (`KismetMathLibrary.MakeVector` 0.0 0.0 (`self.BopFloatUp`)))
          (set `self.UpCounter` (+ (`self.UpCounter`) 1))
          (else
            (`self.K2_AddActorLocalOffset` (`KismetMathLibrary.MakeVector` 0.0 0.0 (`self.BopFloatDown`)))
            (bind _output_get (set `self.DownCounter` (+ (`self.DownCounter`) 1)))
            (if (== _output_get 100)
              (`|ExecutionSequence`
                (:`then_0`
                  (set `self.UpCounter` 0))
                (:`then_1`
                  (set `self.DownCounter` 0))))))))
    (:`then_1`
      ;[1 1 1] Move the enemy towards the player
      (`self.K2_SetActorLocation` (+ (* (* (`KismetMathLibrary.Normal` (- (`self.K2_GetActorLocation` (`GameplayStatics.GetPlayerPawn` 0)) _returnvalue)) (`self.Tick`)) (`self.Speed`)) _returnvalue)))))

(fn `UserConstructionScript`)