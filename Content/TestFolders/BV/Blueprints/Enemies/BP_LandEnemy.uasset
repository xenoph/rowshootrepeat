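; Land-based enemy that turns to face the player (BP_Character), fires projectiles at it and strafes sideways.
; Tick re-aims on a delay, traces forward, and on any hit with the player in FireRange spawns BP_Projectile_LandEnemy after FireRate, scaling velocity by distance and height.
; MoveLeft and MoveRight step only while a side trace hits, with tap flags and a counter alternating direction.
; Without a valid player, it retries the search after a delay.
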(event `FindPlayer`
  ;[1 1 1] Get reference to player (or boat)
  (bind _outactors (`GameplayStatics.GetAllActorsOfClass` "/Game/TestFolders/BV/Blueprints/Character/BP_Character.BP_Character_C" :!label _label))
  (for _array_element _outactors
    (set `self.Player` _array_element)
    (set `self.HasFoundPlayer` true)))

(event `self.ReceiveBeginPlay`
  (`|ExecutionSequence`
    (:`then_0`
      (goto _label))))

(event `self.ReceiveTick`
  (params (DeltaSeconds :type "Float (single-precision)"))
  (bind (_returnvalue_x _returnvalue_y _returnvalue_z) (`KismetMathLibrary.BreakVector` (`self.K2_GetActorLocation`)))
  (bind _staticmesh (`self.StaticMesh`))
  (bind _player (`self.Player`))
  (bind _returnvalue (`SceneComponent.K2_GetComponentLocation` _staticmesh))
  (bind (_returnvalue_roll _returnvalue_pitch _returnvalue_yaw) (`KismetMathLibrary.BreakRotator` (`KismetMathLibrary.FindLookAtRotation` (`self.K2_GetActorLocation`) (`self.K2_GetActorLocation` (`self.Player`)))))
  (if (`KismetSystemLibrary.IsValid` (`self.Player`))
    (`|ExecutionSequence`
      (:`then_0`
        ;[1 1 1] Every .2 seconds, look at the target.
        (`KismetSystemLibrary.Delay` 0.2)
        (if (`self.HasFoundPlayer`)
          (`self.K2_SetActorRotation` (`KismetMathLibrary.MakeRotator` _returnvalue_roll 0.0 _returnvalue_yaw))))
      (:`then_1`
        (if (`self.HasFoundPlayer`)
          (`|ExecutionSequence`
            (:`then_0`
              ;[1 1 1] Trace towards the player. Currently in a straight line.
              (bind (_outhit _returnvalue_2) (`KismetSystemLibrary.LineTraceSingle` :`Start` _returnvalue :`End` (+ _returnvalue (* (`SceneComponent.GetForwardVector` _staticmesh) 2000.0)) :`TraceChannel` "TraceTypeQuery1" :`DrawDebugType` "ForOneFrame" :`TraceColor` (struct :`R` 1.0 :`G` 0.983531 :`B` 0.962442 :`A` 1.0))))
            (:`then_1`
              (if (and _returnvalue_2 (< (/ (`KismetMathLibrary.VSize` (- (`self.K2_GetActorLocation`) (`self.K2_GetActorLocation` (`self.Player`)))) 10.0) (`self.FireRange`)))
                ;[1 1 1] Spawn a projectile, and send it towards the target. Currently not calculating where the player is going.
                (`KismetSystemLibrary.Delay` (`self.FireRate`))
                (bind _returnvalue_3 (`|SpawnActorFromClass` "/Game/TestFolders/BV/Blueprints/Enemies/BP_Projectile_LandEnemy.BP_Projectile_LandEnemy_C" (`KismetMathLibrary.Conv_VectorToTransform` (+ (`self.K2_GetActorLocation`) (`self.GetActorForwardVector`))) "Undefined" "OverrideRootScale"))
                (`ProjectileMovementComponent.SetVelocityInLocalSpace` (`/Game/TestFolders/BV/Blueprints/Enemies/BP_Projectile_LandEnemy.ProjectileMovement` _returnvalue_3) (+ (* (`SceneComponent.GetForwardVector` (`self.Sphere`)) (- (`KismetMathLibrary.VSize` (- (`self.K2_GetActorLocation`) (`self.K2_GetActorLocation` _player))) (* _returnvalue_z 0.5))) (* (`self.GetActorForwardVector` _player) 1.8))))))))
      (:`then_2`
        (if (`self.TapLeft`)
          (`self.MoveLeft`)))
      (:`then_3`
        (if (`self.TapRight`)
          (`self.MoveRight`)))
      (:`then_4`
        (if (or (`self.TappedLeft`) (`self.TappedRight`))
          (bind _output_get (set `self.TapSoFar` (- (`self.TapSoFar`) 2.0)))
          (if (<= _output_get 0.0)
            (if (`self.TappedLeft`)
              (set `self.TapRight` true)
              (set `self.TappedLeft` false)
              (else
                (set `self.TapLeft` true)
                (set `self.TappedRight` false)))))))
    (else
      (`KismetSystemLibrary.Delay` 2.0)
      (`self.FindPlayer`))))

(fn `UserConstructionScript`)