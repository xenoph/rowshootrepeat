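; Health orb pickup that homes in on the player and grants a percentage of health on overlap.
; The orb waits until it is near its BeginPlay X/Y at world height 150, then disables physics and switches to query-only collision.
; Tick then moves the actor toward the player, accelerating each frame when close and using a distance-reduced speed limit when far.
; Sphere overlap with the player calls BP_Character's GetHealthPickup and destroys the orb.
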(event `self.ReceiveBeginPlay`
  (bind (_returnvalue_x _returnvalue_y) (`KismetMathLibrary.BreakVector` (`SceneComponent.K2_GetComponentLocation` (`self.Orb`))))
  (set `self.TargetHeight` (`KismetMathLibrary.MakeVector` _returnvalue_x _returnvalue_y 150.0)))

(event `self.ReceiveTick`
  (params (DeltaSeconds :type "Float (single-precision)"))
  (bind _returnvalue (`self.K2_GetActorLocation`))
  (bind _orb (`self.Orb`))
  (bind _lengthtoplayer (`self.LengthToPlayer`))
  (bind _returnvalue_2 (- (`self.K2_GetActorLocation` (`GameplayStatics.GetPlayerPawn` 0)) _returnvalue))
  (set `self.Tick` DeltaSeconds)
  (if (`self.MoveTowards`)
    (set `self.LengthToPlayer` (`KismetMathLibrary.VSize` _returnvalue_2))
    (`self.K2_SetActorLocation` (+ (* (* (`KismetMathLibrary.Normal` _returnvalue_2) (`self.Tick`)) (`self.Speed`)) _returnvalue))
    (if (< _lengthtoplayer 1500.0)
      (set `self.Speed` (+ (`self.Speed`) 20.0))
      (else
        (set `self.Speed` (- (`self.SpeedLimit`) (/ _lengthtoplayer 100.0)))))
    (elif (not (!= (`SceneComponent.K2_GetComponentLocation` (`self.Orb`)) (`self.TargetHeight`) :`ErrorTolerance` 25.0))
      (set `self.MoveTowards` true)
      (`|ExecutionSequence`
        (:`then_0`
          (`PrimitiveComponent.SetEnableGravity` _orb false))
        (:`then_1`
          (`PrimitiveComponent.SetSimulatePhysics` _orb false))
        (:`then_2`
          (`PrimitiveComponent.SetCollisionEnabled` _orb "QueryOnly")
          (set `PrimitiveComponent.bGenerateOverlapEvents` true (`self.Orb`)))))))

(event `self.Sphere.OnComponentBeginOverlap`
  (params (OverlappedComponent :type "PrimitiveComponent Object Reference") (OtherActor :type "Actor Object Reference") (OtherComp :type "PrimitiveComponent Object Reference") (OtherBodyIndex :type Integer) (bFromSweep :type Boolean) (SweepResult :type "HitResult Structure (by ref)"))
  (if (== OtherActor (`GameplayStatics.GetPlayerPawn` 0))
    (`|ExecutionSequence`
      (:`then_0`
        (bind _asbp_character (cast `/Game/TestFolders/BV/Blueprints/Character/BP_Character` (`GameplayStatics.GetPlayerPawn` 0)))
        (`/Game/TestFolders/BV/Blueprints/Character/BP_Character.GetHealthPickup` _asbp_character (`self.HealthPercentageGiven`)))
      (:`then_1`
        (`self.K2_DestroyActor`)))))

(fn `UserConstructionScript`)