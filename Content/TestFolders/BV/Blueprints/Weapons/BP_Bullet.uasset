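; BP_Bullet is a weapon projectile that damages or destroys enemies on hit.
; It matches the hit actor's class against three types, destroying land enemies and their projectiles outright along with itself.
; Flying enemies lose Health by Damage and spawn a burst of small hurt cubes at the bullet's mesh.
; The bullet destroys itself only on kills, surviving non-lethal and unlisted hits, and prints debug text on every hit.
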(event `self.ReceiveBeginPlay`
  (`/Engine/EditorBlueprintResources/StandardMacros.NegateFloat` (`self.Damage`)))

(event `self.ReceiveActorBeginOverlap`
  (params (OtherActor :type "Actor Object Reference")))

(event `self.ReceiveHit`
  (params (MyComp :type "PrimitiveComponent Object Reference") (Other :type "Actor Object Reference") (OtherComp :type "PrimitiveComponent Object Reference") (bSelfMoved :type Boolean) (HitLocation :type "Vector Structure") (HitNormal :type "Vector Structure") (NormalImpulse :type "Vector Structure") (Hit :type "HitResult Structure (by ref)"))
  (`KismetSystemLibrary.PrintString` "Hello")
  (bind _output_get (set `self.HitObject` Other))
  (for _array_element (`|MakeArray` "/Game/TestFolders/BV/Blueprints/Enemies/FlyingEnemy/FlyingEnemy_Character.FlyingEnemy_Character_C" "/Game/TestFolders/BV/Blueprints/Enemies/LandEnemy/BP_Projectile_LandEnemy.BP_Projectile_LandEnemy_C" "/Game/TestFolders/BV/Blueprints/Enemies/BP_LandEnemy.BP_LandEnemy_C" :!type "Object Class Reference")
    (bind _returnvalue (`GameplayStatics.GetObjectClass` _output_get))
    (if (== _array_element _returnvalue)
      (if (== _returnvalue "/Game/TestFolders/BV/Blueprints/Enemies/FlyingEnemy/FlyingEnemy_Character.FlyingEnemy_Character_C")
        (bind _asflying_enemy_character (cast `/Game/TestFolders/BV/Blueprints/Enemies/FlyingEnemy/FlyingEnemy_Character` (`self.HitObject`)))
        (bind _output_get_2 (set `/Game/TestFolders/BV/Blueprints/Enemies/FlyingEnemy/FlyingEnemy_Character.Health` (- (`/Game/TestFolders/BV/Blueprints/Enemies/FlyingEnemy/FlyingEnemy_Character.Health` _asflying_enemy_character) (`self.Damage`)) _asflying_enemy_character))
        (if (<= _output_get_2 0.0)
          (`|ExecutionSequence`
            (:`then_0`
              (bind _asflying_enemy_character_2 (cast `/Game/TestFolders/BV/Blueprints/Enemies/FlyingEnemy/FlyingEnemy_Character` (`self.HitObject`) :!label _label))
              (for _ (range 11)
                (bind _returnvalue_2 (`|SpawnActorFromClass` "/Game/TestFolders/BV/Blueprints/Enemies/FlyingEnemy/BP_FlyingEnemy_HurtCube.BP_FlyingEnemy_HurtCube_C" (`KismetMathLibrary.Conv_VectorToTransform` (`SceneComponent.K2_GetComponentLocation` (`self.StaticMeshComponent`))) "Undefined" "OverrideRootScale"))
                (`self.SetActorScale3D` _returnvalue_2 (0.1 0.1 0.1))))
            (:`then_1`
              (`self.K2_DestroyActor` (`self.HitObject`))
              (`self.K2_DestroyActor`)))
          (else
            (goto _label)))
        (else
          (`|ExecutionSequence`
            (:`then_0`
              (`self.K2_DestroyActor` (`self.HitObject`)))
            (:`then_1`
              (`self.K2_DestroyActor`))))))))

(fn `UserConstructionScript`)