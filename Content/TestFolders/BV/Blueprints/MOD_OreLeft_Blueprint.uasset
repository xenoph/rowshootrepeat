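; Left oar actor for BP_Boat that turns its own rotation into forward propulsion of the boat.
; On BeginPlay it finds the boat and snaps itself onto the boat's static mesh, keeping relative rotation.
; A Delay on Tick samples yaw about every half second, and CalculateRotationDiff yields a difference only when yaw has decreased.
; That difference scales a mass-independent force along the boat mesh's forward vector.
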(event `self.ReceiveBeginPlay`
  (bind (_returnvalue_roll _returnvalue_pitch _returnvalue_yaw) (`KismetMathLibrary.BreakRotator` (`self.K2_GetActorRotation`)))
  (bind _output_get (set `self.PreviousZRotation` _returnvalue_yaw))
  (bind _output_get_2 (set `self.FirstRotCheck` true))
  (bind _outactors (`GameplayStatics.GetAllActorsOfClass` "/Game/TestFolders/BV/Blueprints/BP_Boat.BP_Boat_C"))
  (for _array_element _outactors
    (bind _output_get_3 (set `self.Boat` _array_element))
    (bind _output_get_4 (set `self.BoatMesh` (`self.GetComponentByClass` _output_get_3 "/Script/Engine.StaticMeshComponent")))
    (`self.K2_AttachToComponent` _output_get_4 "None" "SnapToTarget" "KeepRelative" "KeepRelative" true)))

(event `self.ReceiveTick`
  (params (DeltaSeconds :type "Float (single-precision)"))
  (bind (_returnvalue_roll _returnvalue_pitch _returnvalue_yaw) (`KismetMathLibrary.BreakRotator` (`self.K2_GetActorRotation`)))
  (bind _boatmesh (`self.BoatMesh`))
  (`KismetSystemLibrary.Delay` 0.5)
  (if (stale `self.ReceiveBeginPlay` _output_get_2)
    (set `self.PreviousZRotation` (stale `self.ReceiveBeginPlay` _output_get))
    (set `self.CurrentZRotation` _returnvalue_yaw)
    (set `self.FirstRotCheck` false)
    (else
      (bind _output_get (set `self.PreviousZRotation` (`self.CurrentZRotation`)))
      (bind _output_get_2 (set `self.CurrentZRotation` _returnvalue_yaw))
      (bind _diff (`self.CalculateRotationDiff` _output_get _output_get_2))
      (`PrimitiveComponent.AddForce` _boatmesh (* (`SceneComponent.GetForwardVector` _boatmesh) (* 1200 _diff)) "None" true))))

(fn `CalculateRotationDiff`
  (params (FirstRot :type "Float (double-precision)") (SecondRot :type "Float (double-precision)"))
  (returns (Diff :type "Float (double-precision)"))
  (`/Engine/EditorBlueprintResources/StandardMacros.CompareFloat` FirstRot SecondRot
    (:`>`
      (bind _result (`/Engine/EditorBlueprintResources/StandardMacros.NegateFloat` FirstRot)
        (:`  `
          (bind _result_2 (`/Engine/EditorBlueprintResources/StandardMacros.NegateFloat` SecondRot)
            (:`  `
              (set `self.DiffOutValue` (- _result _result_2)))))))
    (:`==`
      (set `self.DiffOutValue` 0.0))
    (:`<`
      (set `self.DiffOutValue` 0.0)))
  (return (`self.DiffOutValue`)))

(fn `UserConstructionScript`)