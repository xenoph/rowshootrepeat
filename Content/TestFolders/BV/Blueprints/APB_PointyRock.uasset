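; APB_PointyRock is a physics-driven rock actor that shoots upward on spawn, then falls and removes itself.
; BeginPlay derives a target height from the actor's bounds and applies a single mass-independent upward force to the PointyRock component.
; Tick detects arrival near that height, raises angular damping and enables gravity.
; After a delay, it unpauses the Spawner's timer and destroys the actor.
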(event `self.ReceiveBeginPlay`
  ;[1 1 1] On spawn, set the target height and give the object force upwards
  (bind _output_get (set `self.SpawnPosition` (`self.K2_GetActorLocation`)))
  (set `self.TargetHeight` (`KismetMathLibrary.MakeVector` (.x _output_get) (.y _output_get) (+ (.z _output_get) (- (* (.z (`.BoxExtent` (`self.GetActorBounds` false))) 2.0) 50.0))))
  (`PrimitiveComponent.AddForce` (`self.PointyRock`) (0.0 0.0 25000.0) "None" true))

(event `self.ReceiveTick`
  (params (DeltaSeconds :type "Float (single-precision)"))
  (bind _pointyrock (`self.PointyRock`))
  ;[1 1 1] Check if it has reached target height
  (if (not (!= (`SceneComponent.K2_GetComponentLocation` (`self.PointyRock`)) (`self.TargetHeight`) :`ErrorTolerance` 25.0))
    ;[1 1 1] Turn on damping and enable gravity so it will fall down again.
    (`|ExecutionSequence`
      (:`then_0`
        (`PrimitiveComponent.SetAngularDamping` _pointyrock 8.0))
      (:`then_1`
        (`PrimitiveComponent.SetEnableGravity` _pointyrock true)
        (`KismetSystemLibrary.Delay` 5.0)
        (`|ExecutionSequence`
          (:`then_0`
            (`/Game/TestFolders/BV/Triggers/ABP_PointyRockSpawnpoint.UnpauseTimer` (`self.Spawner`)))
          (:`then_1`
            (`self.K2_DestroyActor`)))))))

(fn `UserConstructionScript`)