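; BP_GameMode is a game mode that respawns the player and a boat when the player's character is destroyed.
; On BeginPlay it binds RespawnPlayer to the destroyed event of the current BP_Character.
; After a short delay, RespawnPlayer spawns a BP_NewBoat and a BP_Character at stored spawn transforms, possesses the character, then calls Respawn to rebind the event for the next death.
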(event `Respawn`
  (bind _asbp_character (cast `/Game/TestFolders/BV/Characters/BP_Character` (`GameplayStatics.GetPlayerCharacter` 0) :!label _label))
  (add `self.OnDestroyed` _asbp_character (delegate `RespawnPlayer`)))

(event `self.ReceiveBeginPlay`
  (goto _label))

(event `RespawnPlayer` :!signature `self.OnDestroyed`
  (params (DestroyedActor :type "Actor Object Reference"))
  (`KismetSystemLibrary.Delay` 1.0)
  (`|SpawnActorFromClass` "/Game/TestFolders/BV/Blueprints/BP_NewBoat.BP_NewBoat_C" (`self.SpawnPointBoat`) "Undefined" "OverrideRootScale")
  (bind _returnvalue (`|SpawnActorFromClass` "/Game/TestFolders/BV/Characters/BP_Character.BP_Character_C" (`self.SpawnPointPlayer`) "Undefined" "OverrideRootScale"))
  (`Controller.Possess` (`GameplayStatics.GetPlayerController` 0) _returnvalue)
  (`self.Respawn`))

(fn `UserConstructionScript`)