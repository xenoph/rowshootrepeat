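; Right-side oar actor (named "OreRight") that attaches to the BP_Boat static mesh and turns its own rotation into boat propulsion.
; A Delay on Tick samples actor yaw about every half second, with ValidateValue clamping later samples to a symmetric limit.
; CalculateRotationDiff yields a difference only for increasing yaw, which scales a mass-independent world Y-axis force on the boat mesh.
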(event `self.ReceiveBeginPlay`
  (bind (_returnvalue_roll _returnvalue_pitch _returnvalue_yaw) (`KismetMathLibrary.BreakRotator` (`self.K2_GetActorRotation`)))
  (bind _output_get (set `self.PreviousZRotation` _returnvalue_yaw))
  (bind _output_get_2 (set `self.FirstRotCheck` true))
  (bind _outactors (`GameplayStatics.GetAllActorsOfClass` "/Game/TestFolders/BV/Blueprints/BP_Boat.BP_Boat_C"))
  (for _array_element _outactors
    (bind _output_get_3 (set `self.Boat` _array_element))
    (bind _output_get_4 (set `self.BoatMesh` (`self.GetComponentByClass` _output_get_3 "/Script/Engine.StaticMeshComponent")))
    (`self.K2_AttachToComponent` _output_get_4 "None" "SnapToTarget" "KeepRelative" "KeepRelative" true)))

(event `self.ReceiveTick`
  (params (DeltaSeconds :type "Float (single-precision)"))
  (bind (_returnvalue_roll _returnvalue_pitch _returnvalue_yaw) (`KismetMathLibrary.BreakRotator` (`self.K2_GetActorRotation`)))
  (`KismetSystemLibrary.Delay` 0.5)
  (if (stale `self.ReceiveBeginPlay` _output_get_2)
    (set `self.PreviousZRotation` (stale `self.ReceiveBeginPlay` _output_get))
    (set `self.CurrentZRotation` _returnvalue_yaw)
    (set `self.FirstRotCheck` false)
    (else
      (bind _outvalue (`self.ValidateValue` _returnvalue_yaw))
      (bind _output_get (set `self.PreviousZRotation` (`self.CurrentZRotation`)))
      (bind _output_get_2 (set `self.CurrentZRotation` _outvalue))
      (if (not (== _output_get _output_get_2))
        (bind _diff (`self.CalculateRotationDiff` _output_get _output_get_2))
        (`PrimitiveComponent.AddForce` (`self.BoatMesh`) (`KismetMathLibrary.MakeVector` 0.0 (* 1200 _diff)) "None" true)))))

(fn `CalculateRotationDiff`
  (params (FirstRot :type "Float (double-precision)") (SecondRot :type "Float (double-precision)"))
  (returns (Diff :type "Float (double-precision)"))
  (`/Engine/EditorBlueprintResources/StandardMacros.CompareFloat` FirstRot SecondRot
    (:`>`
      (set `self.DiffOutValue` 0.0))
    (:`==`
      (set `self.DiffOutValue` 0.0))
    (:`<`
      (bind _result (`/Engine/EditorBlueprintResources/StandardMacros.NegateFloat` FirstRot)
        (:`  `
          (bind _result_2 (`/Engine/EditorBlueprintResources/StandardMacros.NegateFloat` SecondRot)
            (:`  `
              (bind _result_3 (`/Engine/EditorBlueprintResources/StandardMacros.NegateFloat` (- _result _result_2))
                (:`  `
                  (set `self.DiffOutValue` _result_3)))))))))
  (return (`self.DiffOutValue`)))

(fn `UserConstructionScript`)

(fn `ValidateValue`
  (params (Value :type "Float (double-precision)"))
  (returns (OutValue :type "Float (double-precision)"))
  (`/Engine/EditorBlueprintResources/StandardMacros.CompareFloat` Value
    (:`>`
      (if (> Value 40.0)
        (set `self.OutValue` 40.0)
        (else
          (set `self.OutValue` Value :!label _label))))
    (:`==`
      (goto _label))
    (:`<`
      (if (< Value -40.0)
        (set `self.OutValue` -40.0)
        (else
          (goto _label)))))
  (return (`self.OutValue`)))