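; BP_Projectile_LandEnemy is a fireball projectile for the land enemy that damages the player.
; On BeginPlay it sets a short lifespan and attaches a fire emitter to its mesh.
; Tick polls the distance to the player and, within a fixed radius, spawns an explosion, calls TakeDamage on BP_Character and destroys itself.
; Hit and overlap events do nothing, so detonation relies on proximity alone; their old explosion logic is left unwired.
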(event `self.ReceiveBeginPlay`
  (`|ExecutionSequence`
    (:`then_0`
      (`self.SetLifeSpan` 4.0))
    (:`then_1`
      ;[1 1 1] Create a fireball effect
      (bind _returnvalue (`GameplayStatics.SpawnEmitterAttached` "/Game/StarterContent/Particles/P_Fire.P_Fire" (`self.StaticMesh`) "None" (0.0 0.0 0.0) (struct) "SnapToTarget" false)))))

(event `self.ReceiveTick`
  (params (DeltaSeconds :type "Float (single-precision)"))
  (bind _returnvalue (`self.K2_GetActorLocation`))
  (if (< (`KismetMathLibrary.VSize` (- _returnvalue (`self.K2_GetActorLocation` (`GameplayStatics.GetPlayerCharacter` 0)))) 400.0)
    (`GameplayStatics.SpawnEmitterAtLocation` "/Game/StarterContent/Particles/P_Explosion.P_Explosion" _returnvalue)
    ;[1 1 1] Deal damage to player
    (bind _asbp_character (cast `/Game/TestFolders/BV/Characters/BP_Character` (`GameplayStatics.GetPlayerCharacter` 0)))
    (`/Game/TestFolders/BV/Characters/BP_Character.TakeDamage` _asbp_character (`self.Damage`))
    (`self.K2_DestroyActor`)))

(event `self.StaticMesh.OnComponentHit`
  (params (HitComponent :type "PrimitiveComponent Object Reference") (OtherActor :type "Actor Object Reference") (OtherComp :type "PrimitiveComponent Object Reference") (NormalImpulse :type "Vector Structure") (Hit :type "HitResult Structure (by ref)")))

(event `self.ReceiveHit`
  (params (MyComp :type "PrimitiveComponent Object Reference") (Other :type "Actor Object Reference") (OtherComp :type "PrimitiveComponent Object Reference") (bSelfMoved :type Boolean) (HitLocation :type "Vector Structure") (HitNormal :type "Vector Structure") (NormalImpulse :type "Vector Structure") (Hit :type "HitResult Structure (by ref)")))

(event `self.ReceiveActorBeginOverlap`
  (params (OtherActor :type "Actor Object Reference"))
  (if (!= OtherActor "/Game/TestFolders/BV/Characters/LandEnemy/LandEnemy_Character.LandEnemy_Character")
    _))

(fn `UserConstructionScript`)